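; BP_CChest is an interactable chest actor whose Interact event currently only prints a debug string identifying it as a chest.
; Its construction script pushes the Emissive value into the lid mesh materials.
; Unconnected logic, which never runs, checks an action component's gameplay tags for a required key and uses a FlipFlop-driven timeline to open or close the lid, activating particles once opened.
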(event EventBeginPlay)

(event Collision|EventActorBeginOverlap
  (params (OtherActor :type Actor%20Object%20Reference)))

(event EventTick
  (params (DeltaSeconds :type Float%20%28single-precision%29)))

(event EventInteract
  (params (InstigatorPawn :type Pawn%20Object%20Reference))
  (Development|PrintString "상자다"))

(fn ConstructionScript
  (Rendering|Material|SetVectorParameterValueonMaterials (Variables|Default|GetLidMesh) "Emissive" (Math|Conversions|ToVector(LinearColor) (Variables|Default|GetEmissive))))